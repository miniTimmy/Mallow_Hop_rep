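; Collectable pickup that homes in on the player and grants one cookie to BP_MallowCharacter on touch.
; Collect calls StartLerping, which starts a fast looping timer on LerpToPlayer once; repeat calls clear that timer without restarting it.
; LerpToPlayer moves the actor toward player pawn 0 by delta time and LerpPower, ignoring the passed target.
; Sphere overlap clears the timer, awards the cookie and destroys the actor.
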(event `self.Sphere1.OnComponentBeginOverlap`
  (params (OverlappedComponent :type "PrimitiveComponent Object Reference") (OtherActor :type "Actor Object Reference") (OtherComp :type "PrimitiveComponent Object Reference") (OtherBodyIndex :type Integer) (bFromSweep :type Boolean) (SweepResult :type "HitResult Structure (by ref)"))
  (`/Engine/EditorBlueprintResources/StandardMacros.IsValid` OtherActor
    (:`Is Valid`
      (`KismetSystemLibrary.K2_ClearAndInvalidateTimerHandle` (`self.LerpProcess`))
      (bind _asbp_mallow_character (cast `/Game/Mallow_Character/Blueprints/BP_MallowCharacter` OtherActor))
      (`/Game/Mallow_Character/Blueprints/BP_MallowCharacter.GetCooki` _asbp_mallow_character 1)
      (`self.K2_DestroyActor`))))

(fn `Collect`
  (params (Target :type "Vector Structure"))
  (returns (Dummy :type Boolean))
  (`self.StartLerping` Target)
  (return false))

(fn `Destroy`
  (`KismetSystemLibrary.K2_ClearAndInvalidateTimerHandle` (`self.LerpProcess`))
  (`self.K2_DestroyActor`))

(fn `LerpToPlayer`
  (`self.K2_SetActorLocation` (`KismetMathLibrary.VLerp` (`SceneComponent.K2_GetComponentLocation` (`self.DefaultSceneRoot`)) (`self.K2_GetActorLocation` (`GameplayStatics.GetPlayerPawn` 0)) (* (`GameplayStatics.GetWorldDeltaSeconds`) (`self.LerpPower`)))))

(fn `StartLerping`
  (params (PlayerLocation :type "Vector Structure"))
  (set `self.PlayerLocation` PlayerLocation)
  (`KismetSystemLibrary.K2_ClearAndInvalidateTimerHandle` (`self.LerpProcess`))
  (if (not (`self.StartedLerping`))
    (bind _returnvalue (`KismetSystemLibrary.K2_SetTimer` null "LerpToPlayer" 0.0017 true))
    (set `self.LerpProcess` _returnvalue)
    (set `self.StartedLerping` true)))

(fn `UserConstructionScript`)