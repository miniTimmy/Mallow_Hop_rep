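; BP_Spawner is a trigger that spawns an actor of PointClassToSpawn when the player character begins overlapping its Box.
; SpawnPoints checks that the class is valid, then spawns one instance at the transform of a randomly picked SpawnLocations actor, ignoring collisions.
; Each new overlap spawns again.
; A loop over every valid location remains in the graph but is disconnected, so it never runs.
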(event `self.Box.OnComponentBeginOverlap`
  (params (OverlappedComponent :type "PrimitiveComponent Object Reference") (OtherActor :type "Actor Object Reference") (OtherComp :type "PrimitiveComponent Object Reference") (OtherBodyIndex :type Integer) (bFromSweep :type Boolean) (SweepResult :type "HitResult Structure (by ref)"))
  (if (== OtherActor (`GameplayStatics.GetPlayerCharacter` 0))
    (`self.SpawnPoints`)))

(fn `SpawnPoints`
  (if (`KismetSystemLibrary.IsValidClass` (`self.PointClassToSpawn`))
    ;[1 1 1] LoopBody
    (`|SpawnActorFromClass` (`self.PointClassToSpawn`) (`self.GetTransform` (`|GetArrayItem` (`self.SpawnLocations`) (`KismetMathLibrary.RandomIntegerInRange` 0 (- (`KismetArrayLibrary.Array_Length` (`self.SpawnLocations`)) 1)))) "AlwaysSpawn" "OverrideRootScale" null null)))

(fn `UserConstructionScript`)