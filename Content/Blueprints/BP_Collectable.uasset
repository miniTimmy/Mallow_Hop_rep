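; BP_Collectable is a pickup actor that reappears at a random spot whenever the player touches it.
; On BeginPlay, InitStatue teleports it to a random X/Y position within fixed bounds at a constant height.
; When the player pawn overlaps it, it destroys itself and spawns a fresh copy at its own transform, whose BeginPlay then moves that copy elsewhere.
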(event `self.ReceiveBeginPlay`
  (`self.InitStatue`))

(event `self.ReceiveActorBeginOverlap`
  (params (OtherActor :type "Actor Object Reference"))
  (if (== OtherActor (`GameplayStatics.GetPlayerPawn` 0))
    (`self.K2_DestroyActor`)
    (`|SpawnActorFromClass` "BP_Collectable_C" (`self.GetTransform`) "Undefined" "OverrideRootScale" null null)))

(fn `InitStatue`
  (`self.K2_TeleportTo` (`KismetMathLibrary.MakeVector` (`KismetMathLibrary.RandomFloatInRange` -1800.0 1000.0) (`KismetMathLibrary.RandomFloatInRange` -1400.0 1400.0) 130.0)))

(fn `UserConstructionScript`)