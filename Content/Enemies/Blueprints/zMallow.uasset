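; zMallow is an enemy Blueprint that animates its scale on death and can damage a linked boss when it dies.
; SetForBoss stores the boss reference and turns on the damage flag.
; On death, a bound handler calls HitBoss on that boss if valid, then a timeline drives the actor's scale and destroys it when finished.
; Nodes that would disable capsule and overlap collision are present but never run.
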(event `self.ReceiveBeginPlay`
  (`parent.ReceiveBeginPlay`)
  (add `self.OnDeath` (delegate `OnDeath_Event`)))

(event `OnDeath_Event`
  (bind _boss (`self.Boss`))
  (if (`self.DmgBoss`)
    (`/Engine/EditorBlueprintResources/StandardMacros.IsValid` _boss
      (:`Is Valid`
        (`/Game/Enemies/Blueprints/BP_Boss.HitBoss` _boss)
        (bind (_direction _lerp) (`Timeline|Timeline_0` :!label _label)
          (:`Update`
            (`self.SetActorScale3D` (`KismetMathLibrary.Conv_DoubleToVector` _lerp)))
          (:`Finished`
            (`self.K2_DestroyActor`))))
      (:`Is Not Valid`
        (goto _label)))
    (else
      (goto _label))))

(fn `SetForBoss`
  (params (Boss :type "/Game/Enemies/Blueprints/BP_Boss Object Reference"))
  (set `self.Boss` Boss)
  (set `self.DmgBoss` true))

(fn `UserConstructionScript`)