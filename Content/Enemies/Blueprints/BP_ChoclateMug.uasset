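; BP_ChoclateMug is an enemy Blueprint for a chocolate mug that handles its own death effect.
; It binds to its OnDeath dispatcher on BeginPlay, then plays a timeline that drives the actor's uniform scale and destroys the actor when finished.
; Nodes for disabling capsule and overlap collision are present but disconnected, so they never run.
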(event `self.ReceiveBeginPlay`
  (`parent.ReceiveBeginPlay`)
  (add `self.OnDeath` (delegate `OnDeath_Event`)))

(event `OnDeath_Event`
  (bind (_direction _lerp) (`Timeline|Timeline_0`)
    (:`Update`
      (`self.SetActorScale3D` (`KismetMathLibrary.Conv_DoubleToVector` _lerp)))
    (:`Finished`
      (`self.K2_DestroyActor`))))

(fn `UserConstructionScript`)