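; Candle holder enemy spawner that starts spitting BP_Flame characters once the Mallow character enters its trigger sphere while SetActive is true.
; A looping timer spawns each flame at the Spawn point and launches it with a random horizontal spread and upward push, scaled by ShootStrength.
; End overlap does nothing because the timer-clearing logic is disconnected, so spawning continues after the player leaves.
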(event `self.TriggerSphere.OnComponentBeginOverlap`
  (params (OverlappedComponent :type "PrimitiveComponent Object Reference") (OtherActor :type "Actor Object Reference") (OtherComp :type "PrimitiveComponent Object Reference") (OtherBodyIndex :type Integer) (bFromSweep :type Boolean) (SweepResult :type "HitResult Structure (by ref)"))
  (if (`self.SetActive`)
    (`/Engine/EditorBlueprintResources/StandardMacros.IsValid` OtherActor
      (:`Is Valid`
        (cast `/Game/Mallow_Character/Blueprints/BP_MallowCharacter` OtherActor)
        (bind _returnvalue (`KismetSystemLibrary.K2_SetTimerDelegate` (delegate `SpawnFlames`) (`self.SpawnTime`) true))
        (set `self.TimerStatus` _returnvalue)))))

(event `SpawnFlames`
  (bind _returnvalue (`KismetMathLibrary.RandomFloatInRange` -500.0 500.0))
  (bind _spawn (`self.Spawn`))
  (bind (_returnvalue_location _returnvalue_rotation) (`KismetMathLibrary.BreakTransform` (`SceneComponent.K2_GetComponentToWorld` (`self.Spawn`))))
  (bind (_returnvalue_x _returnvalue_y _returnvalue_z) (`KismetMathLibrary.BreakVector` (`SceneComponent.K2_GetComponentLocation` _spawn)))
  (bind _returnvalue_2 (`|SpawnActorFromClass` "/Game/Enemies/Blueprints/BP_Flame.BP_Flame_C" (`KismetMathLibrary.MakeTransform` _returnvalue_location _returnvalue_rotation) "AdjustIfPossibleButAlwaysSpawn" "OverrideRootScale" null null))
  (bind _output_get (set `self.Enemy` _returnvalue_2))
  (`Character.LaunchCharacter` _output_get (* (- (`KismetMathLibrary.MakeVector` (+ _returnvalue_x _returnvalue) (+ _returnvalue_y _returnvalue) (+ _returnvalue_z 100.0)) (`SceneComponent.K2_GetComponentLocation` _spawn)) (`self.ShootStrength`)) true true))

(event `self.TriggerSphere.OnComponentEndOverlap`
  (params (OverlappedComponent :type "PrimitiveComponent Object Reference") (OtherActor :type "Actor Object Reference") (OtherComp :type "PrimitiveComponent Object Reference") (OtherBodyIndex :type Integer)))

(fn `UserConstructionScript`)