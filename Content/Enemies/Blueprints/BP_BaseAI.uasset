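; Base AI enemy character that tracks health and deals contact damage to living actors its behavior component identifies as enemies.
; Capsule hits send a one-point hit message to those targets, while incoming hits reduce health, then either trigger death or set a damaged flag as knockback.
; It caches its AI controller on BeginPlay, exposes alive and invincibility queries, and provides a helper that turns the mesh toward a target.
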(event `self.ReceiveBeginPlay`
  (bind _asbp_ai_controller (cast `/Game/MuffinWar/Characters/Muffin/AI/BP_AI_Controller` (`AIBlueprintHelperLibrary.GetAIController` self)))
  (set `self.Controller Reference` _asbp_ai_controller))

(event `self.CapsuleComponent.OnComponentHit`
  (params (HitComponent :type "PrimitiveComponent Object Reference") (OtherActor :type "Actor Object Reference") (OtherComp :type "PrimitiveComponent Object Reference") (NormalImpulse :type "Vector Structure") (Hit :type "HitResult Structure (by ref)"))
  (`/Engine/EditorBlueprintResources/StandardMacros.IsValid` OtherActor
    (:`Is Valid`
      (bind _alive (message `/Game/Intefaces/IAttackable.IsAlive` OtherActor))
      (if _alive
        (if (`/Game/Enemies/Components/BPC_Behavior.IsEnemy` (`self.BPC_Behavior`) OtherActor)
          (message `/Game/Intefaces/IAttackable.HandleHit` OtherActor 1))))))

(fn `Check_If_Dead`
  (if (<= (`self.Health`) 0)
    (set `self.IsAlive_` false)
    (`self.OnDeath`)
    (return)
    (else
      (`self.HandleKnockback`)
      (return))))

(fn `HandleHit`
  (params (Damage :type Integer))
  (returns (Dummy :type Boolean))
  (`self.Take_Dmg` Damage)
  (`self.Check_If_Dead`)
  (return false))

(fn `HandleKnockback`
  (set `self.GetDamaged` true))

(fn `Invicible`
  (returns (Invicible :type Boolean))
  (return (`self.Invicible_`)))

(fn `IsAlive`
  (returns (Alive :type Boolean))
  (return (`self.IsAlive_`)))

(fn `RotateToPlayer`
  (params (RotateToTarget :type "Actor Object Reference"))
  (bind (_returnvalue_roll _returnvalue_pitch _returnvalue_yaw) (`KismetMathLibrary.BreakRotator` (`KismetMathLibrary.FindLookAtRotation` (`SceneComponent.K2_GetComponentLocation` (`self.CapsuleComponent`)) (`self.K2_GetActorLocation` RotateToTarget))))
  (`SceneComponent.K2_SetWorldRotation` (`self.Mesh`) (`KismetMathLibrary.MakeRotator` _returnvalue_roll 0.0 _returnvalue_yaw) true false))

(fn `Take_Dmg`
  (params (Dmg :type Integer))
  (set `self.Health` (- (`self.Health`) Dmg)))

(fn `UserConstructionScript`)