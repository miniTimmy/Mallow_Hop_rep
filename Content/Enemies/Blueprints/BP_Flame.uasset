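; BP_Flame is a flame actor, filed under enemies, that removes itself after a set lifetime.
; BeginPlay runs the parent logic, then starts a one-shot LifeTime timer that fires OnDeath_Event.
; That event disables capsule collision and plays the Lerp timeline to animate uniform actor scale, then destroys the actor when the timeline finishes.
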(event `self.ReceiveBeginPlay`
  (`parent.ReceiveBeginPlay`)
  (`KismetSystemLibrary.K2_SetTimerDelegate` (delegate `OnDeath_Event`) (`self.LifeTime`)))

(event `OnDeath_Event`
  (bind _capsulecomponent (`self.CapsuleComponent`))
  (`PrimitiveComponent.SetCollisionResponseToChannel` _capsulecomponent "ECC_Camera" "ECR_Ignore")
  (`PrimitiveComponent.SetCollisionEnabled` _capsulecomponent "NoCollision")
  (bind (_direction _lerp) (`Timeline|Lerp` :!via `PlayFromStart`)
    (:`Update`
      (`self.SetActorScale3D` (`KismetMathLibrary.Conv_DoubleToVector` _lerp)))
    (:`Finished`
      (`self.K2_DestroyActor`))))

(fn `UserConstructionScript`)