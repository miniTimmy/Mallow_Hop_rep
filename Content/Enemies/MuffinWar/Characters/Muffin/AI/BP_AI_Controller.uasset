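; AI controller for Muffin War enemy muffins that runs the BT_Muffin behavior tree and picks a combat target.
; When perception updates and the blackboard's Enemy is not valid, it scans currently perceived actors for a living BP_Muffin and stores the first one found as Enemy.
; A failed cast on a non-muffin actor stops that scan.
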(event `self.ReceiveBeginPlay`
  (`self.RunBehaviorTree` "/Game/Enemies/MuffinWar/Characters/Muffin/AI/BT_Muffin.BT_Muffin"))

(event `self.AIPerception.OnPerceptionUpdated`
  (params (UpdatedActors :type "Array of Actor Object Reference (by ref)"))
  (bind _returnvalue (`AIBlueprintHelperLibrary.GetBlackboard` null))
  (`/Engine/EditorBlueprintResources/StandardMacros.IsValid` (`BlackboardComponent.GetValueAsObject` _returnvalue "Enemy")
    (:`Is Not Valid`
      (for _array_element (`AIPerceptionComponent.GetCurrentlyPerceivedActors` (`self.AIPerception`) null)
        (bind _asbp_muffin (cast `/Game/Enemies/MuffinWar/Characters/Muffin/Blueprints/BP_Muffin` _array_element))
        (if (not (`/Game/Enemies/MuffinWar/Characters/Muffin/Blueprints/BP_Muffin.IsDead` _asbp_muffin))
          (`BlackboardComponent.SetValueAsObject` _returnvalue "Enemy" _asbp_muffin)
          (break))))))

(fn `UserConstructionScript`)