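; Boss audio actor that switches music between a main theme and a boss theme around a boss encounter.
; On BeginPlay it registers itself with BP_MallowGameMode through SaveAudio, then creates and plays the main theme.
; The first BP_MallowCharacter overlap with its Box creates and plays the boss theme and stops the main one, guarded by DoOnce.
; BossDeath stops any valid boss theme and restarts the main theme from a short offset.
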(event `self.Box.OnComponentBeginOverlap`
  (params (OverlappedComponent :type "PrimitiveComponent Object Reference") (OtherActor :type "Actor Object Reference") (OtherComp :type "PrimitiveComponent Object Reference") (OtherBodyIndex :type Integer) (bFromSweep :type Boolean) (SweepResult :type "HitResult Structure (by ref)"))
  (`/Engine/EditorBlueprintResources/StandardMacros.IsValid` OtherActor
    (:`Is Valid`
      (cast `/Game/Mallow_Character/Blueprints/BP_MallowCharacter` OtherActor)
      (`/Engine/EditorBlueprintResources/StandardMacros.DoOnce` false
        (:`Completed`
          (bind _returnvalue (`AddComponent|NODE_AddAudioComponent-1`))
          (bind _output_get (set `self.BossTheme` _returnvalue))
          (`AudioComponent.Play` _output_get 0.0)
          (`AudioComponent.Stop` (stale `self.ReceiveBeginPlay` _output_get_2)))))))

(event `self.ReceiveBeginPlay`
  (bind _asbp_mallow_game_mode (cast `/Game/Blueprints/BP_MallowGameMode` (`GameplayStatics.GetGameMode`)))
  (bind _output_get (set `self.GameMode` _asbp_mallow_game_mode))
  (`/Game/Blueprints/BP_MallowGameMode.SaveAudio` _output_get self)
  (bind _returnvalue (`AddComponent|NODE_AddAudioComponent-0`))
  (bind _output_get_2 (set `self.MainTheme` _returnvalue))
  (`AudioComponent.Play` _output_get_2 0.0))

(event `BossDeath`
  (bind _bosstheme (`self.BossTheme`))
  (`/Engine/EditorBlueprintResources/StandardMacros.IsValid` _bosstheme
    (:`Is Valid`
      (`AudioComponent.Stop` _bosstheme)
      (`AudioComponent.Play` (`self.MainTheme`) 2.0))))

(fn `UserConstructionScript`)